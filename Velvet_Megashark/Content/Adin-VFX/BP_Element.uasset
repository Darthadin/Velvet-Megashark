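; Element pickup actor that rolls a biased random 0/1 vector on BeginPlay and shows it as its core material color.
; When the player's plane hits it, ColorHit plays a sound, copies the vector into the pawn's element charge and tints the UI parameter collection.
; A FlipFlop alternates playing the BurstShell timeline, auto-reversed after a random delay, and reversing it.
; Sphere overlap only flags CanPickUp and prints; the vector math functions are unused.
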(event OnComponentHit(ElementObject)
  (params (HitComponent :type Primitive%20Component%20Object%20Reference) (OtherActor :type Actor%20Object%20Reference) (OtherComp :type Primitive%20Component%20Object%20Reference) (NormalImpulse :type Vector :default "0, 0, 0") (Hit :type Hit%20Result%20Structure%20%28by%20ref%29))
  ;[1 1 1] Element Transform
  (if (== OtherComp (Variables|/Game/Game/Blueprints/BP_FlyingPawn.BP_FlyingPawn_C|GetPlane%20mesh (.AsBP%20Flying%20Pawn (Utilities|Casting|CastToBP_FlyingPawn (Game|Player|GetPlayerPawn 0)))))
    (CallFunction|ColorHit (Variables|Default|GetElement%20Source%20Vector) "/Game/SFX/Gate-Cue.Gate-Cue")
    (Utilities|FlowControl|FlipFlop
      (:A
        (Utilities|FlowControl|Sequence
          (:then_0
            (bind _shell (Timeline|Burst%20Shell PlayFromStart)
              (:Update
                (Rendering|Material|SetScalarParameterValueonMaterials (Variables|Default|GetElement%20Object) "Exposure - Alpha" _shell))))
          (:then_1
            (Utilities|FlowControl|Delay (Math|Random|RandomFloatinRange 8.0 14.0))
            (Timeline|Burst%20Shell ReverseFromEnd))))
      (:B
        (Timeline|Burst%20Shell ReverseFromEnd)))))

(event OnComponentBeginOverlap(Sphere)
  (params (OverlappedComponent :type Primitive%20Component%20Object%20Reference) (OtherActor :type Actor%20Object%20Reference) (OtherComp :type Primitive%20Component%20Object%20Reference) (OtherBodyIndex :type Integer) (bFromSweep :type Boolean) (SweepResult :type Hit%20Result%20Structure%20%28by%20ref%29))
  ;[1 1 1] Set Can Pick Up
  (if (== OtherComp (Variables|/Game/Game/Blueprints/BP_FlyingPawn.BP_FlyingPawn_C|GetPlane%20mesh (.AsBP%20Flying%20Pawn (Utilities|Casting|CastToBP_FlyingPawn (Game|Player|GetPlayerPawn 0)))))
    (Variables|Default|SetCan%20pick%20up? true)
    (Development|PrintString "Hello")))

(event EventBeginPlay
  (bind _element_object (Variables|Default|GetElement%20Object))
  (Variables|Default|SetElement%20Source%20Vector (CallFunction|GenerateElement))
  (bind _returnvalue (Rendering|Material|CreateDynamicMaterialInstance _element_object 1 (Rendering|Material|GetMaterial _element_object 1) "Core" :!class /Script/Engine.PrimitiveComponent))
  (Rendering|Material|SetVectorParameterValue _returnvalue "Element Color" (Math|Conversions|ToLinearColor(Vector) (Variables|Default|GetElement%20Source%20Vector)) :!class /Script/Engine.MaterialInstanceDynamic))

(fn ConstructionScript)

(fn GenerateElement
  (bind _returnvalue (Math|Random|RandomUnitVector))
  (bind _element_bias (Variables|Default|GetElement%20Bias))
  (bind _returnvalue_2 (Math|Vector|ClampVectorSize _element_bias -1.0 1.0))
  (bind _returnvalue_3 (+ _returnvalue _returnvalue_2))
  (bind (_x _y _z) (Math|Vector|BreakVector _returnvalue_3))
  (return (Math|Vector|MakeVector (Math|Conversions|ToFloat(Integer) (Math|Float|Round (Math|Float|Absolute(Float) _x))) (Math|Conversions|ToFloat(Integer) (Math|Float|Round (Math|Float|Absolute(Float) _y))) (Math|Conversions|ToFloat(Integer) (Math|Float|Round (Math|Float|Absolute(Float) _z))))))

(fn ElementFunctions)

(fn ScramblerArray
  (params (Integer :type Integer)))

(fn ComplexPlaneEquation
  (params (Input :type Vector))
  (return (+ Input (/ "1.000000,1.000000,1.000000" Input))))

(fn 2x+1/2
  (params (Input :type Vector))
  (return (- (* Input "2.000000,2.000000,2.000000") (+ Input "0.500000,0.500000,0.500000"))))

(fn X^2-X/2
  (params (Input :type Vector))
  (return (- (* Input Input) (/ Input "2.000000,2.000000,2.000000"))))

(fn X+1/4
  (params (Input :type Vector))
  (return (+ Input "0.250000,0.250000,0.250000")))

(fn X-1/3
  (params (Input :type Vector))
  (return (+ Input "-0.330000,-0.330000,-0.330000")))

(fn A^2+B^2/C^2
  (params (Input :type Vector))
  (bind _returnvalue (* Input "0.000000,1.000000,0.000000"))
  (bind _returnvalue_2 (* Input "1.000000,0.000000, 0"))
  (bind _returnvalue_3 (* Input "0.000000,0.000000,1.000000"))
  (return (/ (+ (* _returnvalue_2 _returnvalue_2) (* _returnvalue _returnvalue)) (* _returnvalue_3 _returnvalue_3))))

(fn ColorHit
  (params (Generated%20Element :type Vector) (Sound%20Cue :type Sound%20Base%20Object%20Reference))
  (Audio|SpawnSoundatLocation Sound%20Cue (Transformation|GetActorLocation) "0, 0, 0" 1.0 1.0 0.0 0 0)
  (bind _output_get (Variables|/Game/Game/Blueprints/BP_FlyingPawn.BP_FlyingPawn_C|SetCurrent%20Element%20Charge (.AsBP%20Flying%20Pawn (Utilities|Casting|CastToBP_FlyingPawn (Game|Player|GetPlayerPawn 0))) Generated%20Element))
  (Rendering|Material|SetVectorParameterValue "/Game/Adin-VFX/UI/MPC_UI.MPC_UI" "Color" (Math|Conversions|ToLinearColor(Vector) _output_get) :!class /Script/Engine.KismetMaterialLibrary))