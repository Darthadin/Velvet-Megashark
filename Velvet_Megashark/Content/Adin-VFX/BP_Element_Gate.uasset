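; Element gate pickup that boosts the flying pawn's light level when the player's plane mesh passes through it.
; On BeginPlay it generates an element vector and applies it as the gate material's color.
; A player overlap fires a particle burst, calls ColorHit with the element and gate sound, then animates material Alpha through a timeline before destroying itself.
; A DoOnce with a two-second delayed reset limits repeated overlap triggers.
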(event OnComponentBeginOverlap(Collision)
  (params (OverlappedComponent :type Primitive%20Component%20Object%20Reference) (OtherActor :type Actor%20Object%20Reference) (OtherComp :type Primitive%20Component%20Object%20Reference) (OtherBodyIndex :type Integer) (bFromSweep :type Boolean) (SweepResult :type Hit%20Result%20Structure%20%28by%20ref%29))
  (bind _returnvalue (Game|Player|GetPlayerPawn 0))
  (bind _asbp_flying_pawn (Utilities|Casting|CastToBP_FlyingPawn _returnvalue))
  (Utilities|FlowControl|Sequence
    (:then_0
      (Utilities|FlowControl|DoOnce false :!label _label
        (:Completed
          (if (== OtherComp (Variables|/Game/Game/Blueprints/BP_FlyingPawn.BP_FlyingPawn_C|GetPlane%20mesh _asbp_flying_pawn))
            (Default|LightLevelBoost _asbp_flying_pawn)
            (Components|Activation|Activate (Variables|Default|GetP_Energy-Burst-Directional) false)
            (Default|ColorHit self (stale EventBeginPlay _output_get) "/Game/SFX/Gate-Cue.Gate-Cue")
            (bind _alpha (Timeline|Timeline PlayFromStart)
              (:Update
                (Rendering|Material|SetScalarParameterValueonMaterials (Variables|Default|GetElement%20Object) "Alpha" _alpha))
              (:Finished
                (Actor|DestroyActor)))))))
    (:then_1
      (Utilities|FlowControl|Delay 2.0)
      (goto _label Reset))))

(event EventBeginPlay
  (bind _output_get (Variables|Default|SetElement%20Source%20Vector (CallFunction|GenerateElement "0, 0, 0")))
  (Rendering|Material|SetVectorParameterValueonMaterials (Variables|Default|GetElement%20Object) "Color" _output_get))

(fn ConstructionScript
  (|CallParentFunction))