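; Test AI character Blueprint with custom events that set its movement speed.
; Walk waits five seconds, then randomly picks stopped, medium or full speed, while Run sets full speed immediately.
; An unconnected chain checks for the player's flying-pawn plane mesh, tints the character with its element color, turns it along the plane's heading with random jitter, then moves it a random distance that way.
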(event Custom|Walk
  (bind _charactermovement (Variables|Character|GetCharacterMovement))
  (Utilities|FlowControl|Delay 5.0)
  (switch int (Math|Random|RandomIntegerinRange 0 2)
    (:0
      (Variables|/Script/Engine.CharacterMovementComponent|SetMaxWalkSpeed _charactermovement 0.0))
    (:1
      (Variables|/Script/Engine.CharacterMovementComponent|SetMaxWalkSpeed _charactermovement 3e+02))
    (:2
      (Variables|/Script/Engine.CharacterMovementComponent|SetMaxWalkSpeed _charactermovement 6e+02))))

(event Custom|Run
  (Variables|/Script/Engine.CharacterMovementComponent|SetMaxWalkSpeed (Variables|Character|GetCharacterMovement) 6e+02))

(fn ConstructionScript)